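; Base enemy character that exposes health, damage and AI-facing queries such as attack target, patrol route, idle ranges and movement speed tiers.
; BPCHealthSystem handles damage and healing, with its death, blocked and damage response delegates bound in the construction script.
; Death unpossesses the AI controller, ragdolls the mesh and sets a short lifespan.
; Damage response branches are empty, and older EnemyHealth and hit-react logic is disconnected, though EnemyHealth getters remain.
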(event Custom|Death
  (bind _mesh (Variables|Character|GetMesh))
  (Pawn|UnPossess (AI|GetAIController self))
  (Physics|SetSimulatePhysics _mesh true)
  (Collision|SetCollisionEnabled _mesh "QueryAndPhysics")
  (Actor|SetLifeSpan 5.0))

(event Custom|Blocked
  (params (CanBeparried :type Boolean))
  (Development|PrintString "Blocked"))

(event Custom|DamageResponse
  (params (EDamageResponse :type EDamageResponse%20Enum :default "NewEnumerator0"))
  (switch Utilities|FlowControl|Switch|SwitchonEDamageResponse EDamageResponse))

(event Game|Damage|EventAnyDamage
  (params (Damage :type Float%20%28single-precision%29) (DamageType :type Damage%20Type%20Object%20Reference) (InstigatedBy :type Controller%20Object%20Reference) (DamageCauser :type Actor%20Object%20Reference)))

(event EventEnemyHeal
  (params (HealPersionTage :type Float%20%28double-precision%29)))

(fn ConstructionScript
  (bind _bpc_healthsystem (Variables|Default|GetBPC_HealthSystem))
  (EventDispatchers|BindEventtoOnDeath _bpc_healthsystem (EventDispatchers|CreateEvent :!event Custom|Death))
  (EventDispatchers|BindEventtoOnBlocked _bpc_healthsystem (EventDispatchers|CreateEvent :!event Custom|Blocked))
  (EventDispatchers|BindEventtoOnDamageResponse _bpc_healthsystem (EventDispatchers|CreateEvent :!event Custom|DamageResponse)))

(fn AttackTarget
  (return self))

(fn GetCurrentHealth
  (return (Variables|/Game/CyberBattleRoyale/DamageSystem/BPC_HealthSystem.BPC_HealthSystem_C|GetHealth (Variables|Default|GetBPC_HealthSystem))))

(fn GetEnemyCurrentHealth
  (return (Variables|Default|GetEnemyHealth)))

(fn GetEnemyMaxHealth
  (return (Variables|Default|GetEnemyMaxHealth)))

(fn GetIdleRange
  (return 8.5e+02 8e+02))

(fn GetMaxHealth
  (return (Variables|/Game/CyberBattleRoyale/DamageSystem/BPC_HealthSystem.BPC_HealthSystem_C|GetMaxHealth (Variables|Default|GetBPC_HealthSystem))))

(fn GetPatrolRoute
  (return (Variables|AI|GetPatrolRoute)))

(fn Heal
  (params (HealAmount :type Float%20%28double-precision%29))
  (bind _updatehealth (Default|Heal (Variables|Default|GetBPC_HealthSystem) HealAmount))
  (return _updatehealth))

(fn SetMovementSpeed
  (params (Speed :type E_MovementSpeed%20Enum :default "NewEnumerator0"))
  (bind _output_get (Variables|/Script/Engine.CharacterMovementComponent|SetMaxWalkSpeed (Variables|Character|GetCharacterMovement) (Utilities|Select :Index Speed :NewEnumerator0 0.0 :NewEnumerator1 1e+02 :NewEnumerator2 2e+02 :NewEnumerator3 5e+02)))
  (return _output_get))

(fn TakeDamage
  (params (DamageInfo :type BPS%20Damage%20Info%20Structure))
  (bind _wasdamaed (Default|TakeDamage (Variables|Default|GetBPC_HealthSystem) DamageInfo))
  (return _wasdamaed))