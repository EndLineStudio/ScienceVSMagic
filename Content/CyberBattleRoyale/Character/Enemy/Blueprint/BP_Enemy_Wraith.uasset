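; Wraith enemy character for the battle royale game, caching its base enemy AI controller and creating a health bar widget on BeginPlay.
; Its attack plays a montage whose notify damages the controller's attack target only if a Visibility line trace finds no hit, signaling attack end on completion or interruption.
; It also maps movement states to walk speeds, supplies attack and defend radii, and defers death, block and damage responses to its parent.
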(event EventDeath
  ;[1 1 1] Parant class
  (|CallParentFunction))

(event EventEnemyAttack
  (bind _notifyname (Animation|Montage|PlayMontage (Variables|Character|GetMesh) "/Game/CyberBattleRoyale/Character/Enemy/Blueprint/Animation/AM_Enemy_Attack.AM_Enemy_Attack")
    (:OnCompleted
      (Default|CallOnAttackEnd :!label _label))
    (:OnInterrupted
      (goto _label))
    (:OnNotifyBegin
      (switch name _notifyname
        (:Fire
          (bind _aicbaseenemy (Variables|Default|GetAICBaseEnemy)
            (:then
              (bind _attack_target (Variables|/Game/CyberBattleRoyale/Character/Enemy/AI/AIC_Base_Enemy.AIC_Base_Enemy_C|GetAttack%20Target _aicbaseenemy)
                (:then
                  (bind _returnvalue (Collision|LineTraceByChannel (Transformation|GetActorLocation) (Transformation|GetActorLocation _attack_target) "TraceTypeQuery1" false 0 "None"))
                  (if (not _returnvalue)
                    (Class|BPIDamagable|TakeDamage(Message) (Variables|/Game/CyberBattleRoyale/Character/Enemy/AI/AIC_Base_Enemy.AIC_Base_Enemy_C|GetAttack%20Target (Variables|Default|GetAICBaseEnemy)) (Utilities|Struct|MakeBPS_DamageInfo 1e+01 "NewEnumerator2" "NewEnumerator1"))))
                (:else)))
            (:else)))))))

(event EventBeginPlay
  (bind _asaic_base_enemy (Utilities|Casting|CastToAIC_Base_Enemy (AI|GetAIController self)))
  (Variables|Default|SetAICBaseEnemy _asaic_base_enemy)
  (CallFunction|SetHealthBarWidget self))

(event EventBlocked
  (params (CanBeparried :type Boolean))
  ;[1 1 1] Parant class
  (|CallParentFunction CanBeparried))

(event EventDamageResponse
  (params (EDamageResponse :type EDamageResponse%20Enum :default "NewEnumerator0"))
  ;[1 1 1] Parant class
  (|CallParentFunction EDamageResponse))

(fn ConstructionScript)

(fn SetMovementSpeed
  (params (Speed :type E_MovementSpeed%20Enum :default "NewEnumerator0"))
  (bind _output_get (Variables|/Script/Engine.CharacterMovementComponent|SetMaxWalkSpeed (Variables|Character|GetCharacterMovement) (Utilities|Select :Index Speed :NewEnumerator0 0.0 :NewEnumerator1 1e+02 :NewEnumerator2 2e+02 :NewEnumerator3 5e+02)))
  (return _output_get))

(fn GetIdleRange
  (return 6e+02 6e+02))

(fn SetHealthBarWidget
  (params (DamagableActor :type BPI%20Damagable%20Interface))
  (bind _returnvalue (UserInterface|CreateWidget "/Game/CyberBattleRoyale/HUD/Health/WB_EnemyHealthBar.WB_EnemyHealthBar_C" 0 DamagableActor))
  (UserInterface|SetWidget (Variables|Default|GetHealthBar) _returnvalue)
  (return))

(fn AttackTarget
  (return self))