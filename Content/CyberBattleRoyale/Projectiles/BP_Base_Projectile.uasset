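; Base projectile actor that flies at a set speed toward a target actor or, without one, a given location.
; The construction script applies speed and gravity to the movement component and enables homing when flagged and a target exists.
; On BeginPlay it ignores its instigator, or owner as fallback, and aims its velocity.
; A box collision hit fires an impact dispatcher, spawns effect and sound, then destroys the projectile.
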(event OnComponentHit(BoxCollision)
  (params (HitComponent :type Primitive%20Component%20Object%20Reference) (OtherActor :type Actor%20Object%20Reference) (OtherComp :type Primitive%20Component%20Object%20Reference) (NormalImpulse :type Vector :default "0, 0, 0") (Hit :type Hit%20Result%20Structure%20%28by%20ref%29))
  (bind _location (Collision|BreakHitResult Hit))
  (Default|CallOnProjectileImpect OtherActor Hit)
  (Effects|SpawnEmitteratLocation (Variables|Effects|GetImpectEffect) _location)
  (Audio|PlaySoundatLocation (Variables|Sounds|GetImpectSound) _location "0, 0, 0" 1.0 1.0 0.0 0 0 0 0)
  (Actor|DestroyActor))

(event Custom|RotateToTarget
  (Variables|/Script/Engine.MovementComponent|SetVelocity (Variables|Default|GetProjectileMovement) (* (Math|Vector|GetUnitDirection(Vector) (Transformation|GetActorLocation) (Transformation|GetActorLocation (Variables|Target|GetTargetPoint))) (Variables|ProjectileSetting|GetSpeed))))

(event EventBeginPlay
  (bind _returnvalue (Game|GetInstigator))
  (Collision|IgnoreActorwhenMoving (Variables|Default|GetBoxCollision) (select (Utilities|IsValid _returnvalue) _returnvalue (Components|GetOwner)) true)
  (Variables|Target|GetTargetPoint
    (:then
      (CallFunction|RotatetoTarget))
    (:else
      (CallFunction|MoveNormal))))

(fn ConstructionScript
  (bind _projectilemovement (Variables|Default|GetProjectileMovement))
  (Variables|/Script/Engine.ProjectileMovementComponent|SetInitialSpeed _projectilemovement (Variables|ProjectileSetting|GetSpeed))
  (Variables|/Script/Engine.ProjectileMovementComponent|SetMaxSpeed _projectilemovement (Variables|ProjectileSetting|GetSpeed))
  (Variables|/Script/Engine.ProjectileMovementComponent|SetProjectileGravityScale _projectilemovement (Variables|ProjectileSetting|GetGravity))
  (Variables|Target|GetTargetPoint
    (:then
      (if (Variables|ProjectileSetting|GetIsHoming)
        (Variables|/Script/Engine.ProjectileMovementComponent|SetbIsHomingProjectile _projectilemovement true)
        (Variables|/Script/Engine.ProjectileMovementComponent|SetHomingTargetComponent _projectilemovement (Variables|/Script/Engine.Actor|GetRootComponent (Variables|Target|GetTargetPoint)))))
    (:else)))

(fn MoveNormal
  (Variables|/Script/Engine.MovementComponent|SetVelocity (Variables|Default|GetProjectileMovement) (* (Math|Vector|GetUnitDirection(Vector) (Transformation|GetActorLocation) (Variables|Default|GetMoveTo)) (Variables|ProjectileSetting|GetSpeed))))