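; Attack component for a battle royale game that provides a projectile base attack, a lightning strike and a targeted heal.
; BaseAttack spawns a dark or light short projectile at a mesh socket by AttackCount, binding its impact to fixed damage.
; LightningStrike spawns a delayed AOE on a target that damages overlapped actors.
; HealTarget line-traces for a spot to trigger a heal AOE, which heals only that target.
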(event Custom|LightningStrike
  (params (AttackTarget :type Actor%20Object%20Reference) (DelayBeforeStrike :type Float%20%28double-precision%29) (Dmg_Ammount :type Float%20%28double-precision%29))
  (bind _returnvalue (Components|GetOwner))
  (bind (_aspawn _bsuccess) (Utilities|Casting|CastToPawn _returnvalue))
  (Utilities|IsValid AttackTarget
    (:Is%20Valid
      (bind _returnvalue_2 (Game|SpawnActorfromClass "/Game/CyberBattleRoyale/Projectiles/BP_AOE_LightStrike.BP_AOE_LightStrike_C" (Math|Transform|MakeTransform "0, 0, 0" "0, 0, 0" "1.000000,1.000000,1.000000") "Undefined" "OverrideRootScale" 0 DelayBeforeStrike AttackTarget "/Game/FXVarietyPack/Particles/P_ky_lightning3.P_ky_lightning3" "/Game/StarterContent/Audio/Explosion01.Explosion01" true false false (select _bsuccess _aspawn 0)))
      (EventDispatchers|AssignOnAOEOverlapActor _returnvalue_2 (delegate Custom|DamageEnemyAOE)))))

(event Custom|HealTarget
  (params (HealTarget :type Actor%20Object%20Reference))
  (bind _returnvalue (Transformation|GetActorLocation HealTarget))
  (Utilities|IsValid HealTarget
    (:Is%20Valid
      (bind (_outhit _returnvalue_2) (Collision|LineTraceByChannel _returnvalue (* _returnvalue "1.000000,1.000000,-1000.000000") "TraceTypeQuery1" false (Utilities|Array|MakeArray HealTarget) "None"))
      (if _returnvalue_2
        (bind _returnvalue_3 (Game|SpawnActorfromClass "/Game/CyberBattleRoyale/Projectiles/BP_AOE_Heal.BP_AOE_Heal_C" (Math|Transform|MakeTransform (.Location (Collision|BreakHitResult _outhit)) "0, 0, 0" "1.000000,1.000000,1.000000") "Undefined" "OverrideRootScale" 0 1.0 5.0 false false false 0))
        (EventDispatchers|AssignOnAOEOverlapActor _returnvalue_3 (delegate Custom|OnHealTarget))
        (Default|Trigger _returnvalue_3)))))

(event Custom|OnHealTarget
  (params (Actor :type Actor%20Object%20Reference))
  (if (== Actor (stale Custom|HealTarget HealTarget))
    (Class|BPIDamagable|Heal(Message) Actor 1e+01)))

(event Custom|BaseAttack
  (params (RootComponent :type Primitive%20Component%20Object%20Reference) (AttackCount :type Integer) (MeshComponent :type Scene%20Component%20Object%20Reference) (InSocketName :type Name) (Target%20Point :type Actor%20Object%20Reference) (MoveTo :type Vector))
  (bind _returnvalue (Transformation|GetSocketTransform MeshComponent InSocketName "RTS_World"))
  (bind _returnvalue_2 (Components|GetOwner))
  (switch int AttackCount
    (:0
      (bind _returnvalue_3 (Game|SpawnActorfromClass "/Game/CyberBattleRoyale/Projectiles/BP_Projectile_DarkShort.BP_Projectile_DarkShort_C" (Math|Transform|MakeTransform (.location _returnvalue) (Math|Rotator|MakeRotator (.roll (.rotation _returnvalue)) 0.0 (.yaw (.rotation _returnvalue))) (.scale _returnvalue)) "Undefined" "OverrideRootScale" _returnvalue_2 1e+03 0.0 Target%20Point false MoveTo 0))
      (CallFunction|BaseAttackBind RootComponent _returnvalue_3)
      (Actor|SetLifeSpan _returnvalue_3 5.0))
    (:1
      (bind _returnvalue_4 (Game|SpawnActorfromClass "/Game/CyberBattleRoyale/Projectiles/BP_Projectile_LightShort.BP_Projectile_LightShort_C" (Math|Transform|MakeTransform (.location _returnvalue) (Math|Rotator|MakeRotator (.roll (.rotation _returnvalue)) 0.0 (.yaw (.rotation _returnvalue))) (.scale _returnvalue)) "Undefined" "OverrideRootScale" _returnvalue_2 1e+03 0.0 Target%20Point false MoveTo 0))
      (CallFunction|BaseAttackBind RootComponent _returnvalue_4)
      (Actor|SetLifeSpan _returnvalue_4 5.0))))

(event Custom|DamageEnemyAOE
  (params (Actor :type Actor%20Object%20Reference))
  (Class|BPIDamagable|TakeDamage(Message) Actor (Utilities|Struct|MakeBPS_DamageInfo (stale Custom|LightningStrike Dmg_Ammount) "NewEnumerator3" "NewEnumerator1")))

(event Custom|BaseAttackBind
  (params (RootComponent :type Primitive%20Component%20Object%20Reference) (Base%20Projecttile :type BP%20Base%20Projectile%20Object%20Reference))
  (EventDispatchers|AssignOnProjectileImpect Base%20Projecttile (delegate Custom|DamageEnemy))
  (Collision|IgnoreActorwhenMoving RootComponent Base%20Projecttile true))

(event Custom|DamageEnemy
  (params (Other%20Actor :type Actor%20Object%20Reference) (Hit :type Hit%20Result%20Structure))
  (Class|BPIDamagable|TakeDamage(Message) Other%20Actor (Utilities|Struct|MakeBPS_DamageInfo 1e+01 "NewEnumerator2" "NewEnumerator1")))