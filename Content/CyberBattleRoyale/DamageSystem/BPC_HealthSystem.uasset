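; Health component that tracks an actor's health, death, blocking, invincibility and interruptibility for the damage system.
; TakeDamage uses CanBeDamaged to sort each damage info into block, damage or no damage, reporting whether damage landed.
; Blocks fire OnBlocked with parry eligibility; lethal hits fire OnDeath, while survivable hits fire OnDamageResponse only when interruptible or force-interrupted.
; Heal adds health clamped to the maximum while the owner is alive.
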(event EventBeginPlay)

(event EventTick
  (params (DeltaSeconds :type Float%20%28single-precision%29)))

(fn Heal
  (params (HealAmount :type Float%20%28double-precision%29))
  (if (not (Variables|Default|GetIsDead))
    (bind _output_get (Variables|Default|SetHealth (Math|Float|Clamp(Float) (+ HealAmount (Variables|Default|GetHealth)) 0.0 (Variables|Default|GetMaxHealth))))
    (return _output_get)))

(fn TakeDamage
  (params (DamageInfo :type BPS%20Damage%20Info%20Structure))
  (bind (_dmg_ammount _dmg_type _dmg_response _shoulddamageinvincible _canbeblocked _canbeparried _shouldforceinterrupt) (Utilities|Struct|BreakBPS_DamageInfo DamageInfo))
  (Utilities|CanbeDamaged _shoulddamageinvincible _canbeblocked
    (:BlockDamage
      (Default|CallOnBlocked _canbeparried)
      (return false))
    (:DoDamage
      (bind _output_get (Variables|Default|SetHealth (- (Variables|Default|GetHealth) _dmg_ammount)))
      (if (<= _output_get 0.0)
        (Variables|Default|SetIsDead true)
        (Default|CallOnDeath)
        (return true)
        (elif (or (Variables|Default|GetIsInterruptible) _shouldforceinterrupt)
          (Default|CallOnDamageResponse _dmg_response)
          (return true))))
    (:NoDamage
      (return false))))